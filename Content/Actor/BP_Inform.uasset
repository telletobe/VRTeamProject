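; BP_Inform is an actor that shows a start widget on its WidgetComponent and swaps it for an information widget when the start button is clicked.
; BeginPlay turns off the component's shadow and binds the start button of WBP_MyStartWidget.
; The click hides the button, then creates, stores and assigns a WBP_Inform to the same component.
; A separate SetVisibility event hides whichever widget the component currently holds.
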(event Custom|SetVisibility
  (Widget|SetVisibility (UserInterface|GetWidget (Variables|Default|GetWidgetComponent)) "Hidden"))

(event Custom|OnClicked_Event
  (Utilities|FlowControl|Sequence
    (:then_0
      (Widget|SetVisibility (Variables|/Game/UMG/WBP_MyStartWidget.WBP_MyStartWidget_C|GetBT_StartButton (stale EventBeginPlay _aswbp_my_start_widget)) "Hidden"))
    (:then_1
      (bind _returnvalue (UserInterface|CreateWidget "/Game/UMG/WBP_Inform.WBP_Inform_C"))
      (bind _output_get (Variables|Default|SetWBP_Inform _returnvalue))
      (UserInterface|SetWidget (Variables|Default|GetWidgetComponent) _output_get))))

(event EventBeginPlay
  (bind _widgetcomponent (Variables|Default|GetWidgetComponent))
  (Rendering|SetCastShadow _widgetcomponent false)
  (bind _aswbp_my_start_widget (Utilities|Casting|CastToWBP_MyStartWidget (UserInterface|GetWidget _widgetcomponent)))
  (EventDispatchers|AssignOnClicked (Variables|/Game/UMG/WBP_MyStartWidget.WBP_MyStartWidget_C|GetBT_StartButton _aswbp_my_start_widget) (delegate Custom|OnClicked_Event)))

(event Collision|EventActorBeginOverlap
  (params (OtherActor :type Actor%20Object%20Reference)))

(event EventTick
  (params (DeltaSeconds :type Float%20%28single-precision%29)))

(fn ConstructionScript)